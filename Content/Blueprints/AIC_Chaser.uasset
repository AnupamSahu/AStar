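; AIC_Chaser is an AI controller meant to move its pawn toward a tagged player along an A* path.
; SolvePath finds the first BP_Player tagged Target, stores AStarPathFinder's route from the pawn to it and raises a travel flag.
; Tick calls TravelPath every frame, but that function is empty, and nothing in this graph calls SolvePath.
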(event EventTick
  (params (DeltaSeconds :type Float%20%28single-precision%29))
  (CallFunction|TravelPath DeltaSeconds))

(fn ConstructionScript)

(fn SolvePath
  (bind _outactors (Actor|GetAllActorsOfClasswithTag "/Game/Blueprints/BP_Player.BP_Player_C" "Target"))
  (if (Utilities|Array|IsValidIndex _outactors)
    (bind _outpath (Class|AStarPathFinder|FindPath (Variables|Default|GetAStarPathFinder) (Transformation|GetActorLocation (Pawn|GetControlledPawn)) (Transformation|GetActorLocation (Utilities|Array|Get(acopy) _outactors))))
    (Variables|Default|SetPath _outpath)
    (Variables|Default|SetShouldTravelPath true)))

(fn TravelPath
  (params (DeltaSeconds :type Float%20%28single-precision%29)))