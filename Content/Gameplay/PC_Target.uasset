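; Player controller that moves its pawn in fixed steps under a fixed overhead camera.
; On BeginPlay it spawns BP_Camera high above the world and makes it the view target.
; Each press of the four Move input actions calls a matching function that offsets the controlled pawn along the world forward or right axis, using SetActorLocation with sweep and teleport enabled.
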(event EventBeginPlay
  (bind _returnvalue (Game|SpawnActorfromClass "/Game/Gameplay/BP_Camera.BP_Camera_C" (Math|Transform|MakeTransform "0,-750.000000,5000.000000" "-90.000000, 0, 0") "Undefined" 0 0))
  (Game|Player|SetViewTargetwithBlend _returnvalue 0.0 "VTBlend_Linear" 0.0 false))

(event Input|ActionEvents|InputActionMoveLeft
  (params (Key :type Key%20Structure :default "None"))
  (:Pressed
    (CallFunction|MoveLeft)))

(event Input|ActionEvents|InputActionMoveRight
  (params (Key :type Key%20Structure :default "None"))
  (:Pressed
    (CallFunction|MoveRight)))

(event Input|ActionEvents|InputActionMoveDown
  (params (Key :type Key%20Structure :default "None"))
  (:Pressed
    (CallFunction|MoveDown)))

(event Input|ActionEvents|InputActionMoveUp
  (params (Key :type Key%20Structure :default "None"))
  (:Pressed
    (CallFunction|MoveUp)))

(fn ConstructionScript)

(fn MoveLeft
  (bind _returnvalue (Pawn|GetControlledPawn))
  (Transformation|SetActorLocation _returnvalue (+ (Transformation|GetActorLocation _returnvalue) (* (Class|KismetMathLibrary|VectorRight) -1e+02)) true true))

(fn MoveRight
  (bind _returnvalue (Pawn|GetControlledPawn))
  (Transformation|SetActorLocation _returnvalue (+ (Transformation|GetActorLocation _returnvalue) (* (Class|KismetMathLibrary|VectorRight) 1e+02)) true true))

(fn MoveUp
  (bind _returnvalue (Pawn|GetControlledPawn))
  (Transformation|SetActorLocation _returnvalue (+ (Transformation|GetActorLocation _returnvalue) (* (Class|KismetMathLibrary|VectorForward) 1e+02)) true true))

(fn MoveDown
  (bind _returnvalue (Pawn|GetControlledPawn))
  (Transformation|SetActorLocation _returnvalue (+ (Transformation|GetActorLocation _returnvalue) (* (Class|KismetMathLibrary|VectorForward) -1e+02)) true true))